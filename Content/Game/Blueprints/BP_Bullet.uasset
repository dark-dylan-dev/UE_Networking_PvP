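; BP_Bullet is a projectile Blueprint for PvP that damages player characters it overlaps and credits the shooter.
; On overlap, it passes its instigator and that pawn's controller to CheckCollision, which ignores the shooter's own character.
; A valid hit calls ApplyDamage on the struck BP_PvP_Character with the shooter's PlayerState and controller, then destroys the bullet.
; Overlaps with other actors do nothing, and a BeginPlay timer destroys the bullet after a fixed lifetime.
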(event OnComponentBeginOverlap(CollisionComponent)
  (params (OverlappedComponent :type Primitive%20Component%20Object%20Reference) (OtherActor :type Actor%20Object%20Reference) (OtherComp :type Primitive%20Component%20Object%20Reference) (OtherBodyIndex :type Integer) (bFromSweep :type Boolean) (SweepResult :type Hit%20Result%20Structure%20%28by%20ref%29))
  (bind _returnvalue (Game|GetInstigator))
  (Utilities|Casting|CastToBP_PvP_Character _returnvalue)
  (bind _asbp_pv_p_controller (Utilities|Casting|CastToBP_PvP_Controller (Pawn|GetController _returnvalue)))
  (CallFunction|CheckCollision _returnvalue OtherActor _asbp_pv_p_controller))

(event Custom|CheckCollision
  (params (Instigator :type Pawn%20Object%20Reference) (OtherActor :type Actor%20Object%20Reference) (InstigatorController :type BP%20Pv%20P%20Controller%20Object%20Reference))
  (bind _asbp_pv_p_character (Utilities|Casting|CastToBP_PvP_Character OtherActor))
  (bind _asbp_pv_p_character_2 (Utilities|Casting|CastToBP_PvP_Character Instigator))
  (if (not (== _asbp_pv_p_character _asbp_pv_p_character_2))
    (bind _asbp_pv_p_player_state (Utilities|Casting|CastToBP_PvP_PlayerState (Variables|/Script/Engine.Pawn|GetPlayerState _asbp_pv_p_character_2)))
    (Utilities|Casting|CastToBP_PvP_Controller (Pawn|GetController Instigator))
    (Default|ApplyDamage _asbp_pv_p_character _asbp_pv_p_player_state InstigatorController)
    (CallFunction|DestroySelf)))

(event EventBeginPlay
  (Utilities|Time|SetTimerbyFunctionName 0 "DestroySelf" 5.0))

(fn ConstructionScript)

(fn DestroySelf
  (Actor|DestroyActor))
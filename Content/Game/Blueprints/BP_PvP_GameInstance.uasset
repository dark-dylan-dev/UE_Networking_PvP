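; PvP game instance that handles LAN multiplayer sessions and keeps the player's chat name across map changes.
; Hosting creates a LAN session and opens the Lobby level.
; Joining only searches: results are stored on BP_PvP_GameState and each becomes a WBP_UniqueSession widget in the controller's found-sessions scroll box.
; The persistent name is set by event and handed back to a controller on request.
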(event Custom|HostSession
  (params (Controller :type BP%20Pv%20P%20Controller%20Object%20Reference))
  (|Session Controller (Variables|Default|GetMAX_PLAYERS) true false
    (:OnSuccess
      (Game|OpenLevel(byName) "Lobby" true "?listen"))))

(event Custom|JoinSession
  (params (Controller :type BP%20Pv%20P%20Controller%20Object%20Reference))
  (bind _results (|FindSessions Controller (Variables|Default|GetMAX_SESSIONS) true false)
    (:OnSuccess
      (bind _asbp_pv_p_game_state (Utilities|Casting|CastToBP_PvP_GameState (Game|GetGameState)))
      (bind _output_get (Variables|/Game/Game/Blueprints/Override/BP_PvP_GameState.BP_PvP_GameState_C|SetGameSessions _asbp_pv_p_game_state _results))
      (for _array_element _output_get
        (bind _returnvalue (UserInterface|CreateWidget "/Game/Game/Blueprints/HUD/WBP_UniqueSession.WBP_UniqueSession_C" Controller))
        (Variables|/Game/Game/Blueprints/HUD/WBP_UniqueSession.WBP_UniqueSession_C|SetSession _returnvalue _array_element)
        (Widget|Panel|AddChild (Variables|/Game/Game/Blueprints/HUD/WBP_FoundSessions.WBP_FoundSessions_C|GetScrollBox (Variables|/Game/Game/Blueprints/Override/BP_PvP_Controller.BP_PvP_Controller_C|GetFoundSessionsHUD_Ref Controller)) _returnvalue)))))

(event Custom|SetPersistentName
  (params (Name :type String))
  ;[0.15 0.15 0.15 0.5] To get the player's name in the chat across different maps using the game instance.
  (Variables|Default|SetPersistentName Name))

(event Custom|GetNameBack
  (params (Controller :type BP%20Pv%20P%20Controller%20Object%20Reference))
  ;[0.15 0.15 0.15 0.5] To get the player's name in the chat across different maps using the game instance.
  (Default|GetNameBack Controller (Variables|Default|GetPersistentName)))
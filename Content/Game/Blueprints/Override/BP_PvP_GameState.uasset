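; PvP match GameState that runs the global countdown and decides the result by kill count when it expires.
; StartTimer arms the Tick countdown, whose GlobalTimer RepNotify calls DecrementTimer on each BP_PvP_Controller.
; EndGame scans player states for Winner and Second, then adds tie screens to both or win and lose screens to all players.
; ChatLog's RepNotify only prints the log, and GlobalCooldown's is empty.
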(event Custom|StartTimer
  (Variables|Default|SetTimerStarted true)
  (Variables|Default|SetGameEnded false))

(event Custom|EndGame
  (bind _returnvalue (Class|GameplayStatics|GetNumPlayerStates))
  (bind _returnvalue_2 (- _returnvalue 1))
  (Variables|Default|SetGameEnded true)
  (for _index (range 0 _returnvalue_2)
    (bind _asbp_pv_p_player_state (Utilities|Casting|CastToBP_PvP_PlayerState (Game|GetPlayerState _index)))
    (if (> (Variables|/Game/Game/Blueprints/Override/BP_PvP_PlayerState.BP_PvP_PlayerState_C|GetKills _asbp_pv_p_player_state) (Variables|Default|GetTopKills))
      (Variables|Default|SetTopKills (Variables|/Game/Game/Blueprints/Override/BP_PvP_PlayerState.BP_PvP_PlayerState_C|GetKills _asbp_pv_p_player_state))
      (Variables|Default|SetWinner _asbp_pv_p_player_state)
      (elif (== (Variables|/Game/Game/Blueprints/Override/BP_PvP_PlayerState.BP_PvP_PlayerState_C|GetKills _asbp_pv_p_player_state) (Variables|Default|GetTopKills))
        (Variables|Default|SetSecond (Variables|Default|GetWinner))
        (else
          (Variables|Default|SetSecond _asbp_pv_p_player_state)))))
  (if (== (Variables|/Game/Game/Blueprints/Override/BP_PvP_PlayerState.BP_PvP_PlayerState_C|GetKills (Variables|Default|GetWinner)) (Variables|/Game/Game/Blueprints/Override/BP_PvP_PlayerState.BP_PvP_PlayerState_C|GetKills (Variables|Default|GetSecond)))
    (Default|AddTieScreen (Variables|Default|GetSecond))
    (else
      (for _index_2 (range 0 _returnvalue_2)
        (bind _asbp_pv_p_player_state_2 (Utilities|Casting|CastToBP_PvP_PlayerState (Game|GetPlayerState _index_2)))
        (if (== _asbp_pv_p_player_state_2 (Variables|Default|GetWinner))
          (Default|AddWinScreen (Variables|Default|GetWinner))
          (else
            (Default|AddLoseScreen _asbp_pv_p_player_state_2)))))))

(event EventTick
  (params (DeltaSeconds :type Float%20%28single-precision%29))
  (if (and (> (Variables|Default|GetGlobalTimer) DeltaSeconds) (Variables|Default|GetTimerStarted))
    (Variables|Default|SetGlobalTimer (- (Variables|Default|GetGlobalTimer) DeltaSeconds))
    (elif (Variables|Default|GetTimerStarted)
      (Variables|Default|SetTimerStarted false)
      (CallFunction|EndGame))))

(fn ConstructionScript)

(fn OnRepGlobalCooldown)

(fn OnRepGlobalTimer
  (for _index (range 0 (- (Class|GameplayStatics|GetNumPlayerControllers) 1))
    (bind _asbp_pv_p_controller (Utilities|Casting|CastToBP_PvP_Controller (Game|GetPlayerController _index)))
    (Default|DecrementTimer _asbp_pv_p_controller)))

(fn OnRepChatLog
  (Development|PrintString (Utilities|String|Append "Chat Log : 
" (Variables|Default|GetChatLog))))
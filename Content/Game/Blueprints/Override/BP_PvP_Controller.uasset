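; PvP player controller that sets up each local player's screen UI by level and handles travel to the Lobby map.
; After a brief delay on BeginPlay, it adds global, user and crosshair widgets in Lobby, or the main HUD in any other level.
; The main HUD's join button triggers a console Travel command to Lobby as a listen map.
; A ServerTravel variant exists but is never run.
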(event Custom|OnPressed_Event
  (CallFunction|ClientTravelLobby))

(event Custom|TravelToGlobal
  (Development|ExecuteConsoleCommand "ServerTravel /Game/Game/Maps/Lobby?listen" self))

(event Custom|ClientTravel_Lobby
  (Development|ExecuteConsoleCommand "Travel /Game/Game/Maps/Lobby?listen" self)
  (Development|PrintString "Hello"))

(event EventBeginPlay
  (|CallParentFunction)
  (Utilities|FlowControl|Delay 0.01)
  (if (Pawn|IsLocalPlayerController)
    (bind _returnvalue (Game|GetCurrentLevelName true))
    (if (Utilities|Enum|Equal(Enum) _returnvalue "Lobby")
      ;[0.15 0.15 0.15 0.5] Add user hud to player screen
      (bind _returnvalue_2 (UserInterface|CreateWidget (Variables|Default|GetGlobal_HUD) self))
      (UserInterface|Viewport|AddtoPlayerScreen _returnvalue_2)
      (bind _returnvalue_3 (UserInterface|CreateWidget (Variables|Default|GetUser_HUD) self))
      (UserInterface|Viewport|AddtoPlayerScreen _returnvalue_3)
      (bind _returnvalue_4 (UserInterface|CreateWidget (Variables|Default|GetUser_Crosshairs) self))
      (UserInterface|Viewport|AddtoPlayerScreen _returnvalue_4)
      (else
        (bind _returnvalue_5 (UserInterface|CreateWidget (Variables|Default|GetMain_HUD) self))
        (bind _output_get (Variables|Default|SetMainMenu_HUD_Ref _returnvalue_5))
        (UserInterface|Viewport|AddtoPlayerScreen _output_get)
        (EventDispatchers|AssignOnPressed (Variables|/Game/Game/Blueprints/HUD/WBP_MainMenu.WBP_MainMenu_C|GetJoinGame_Button (Variables|Default|GetMainMenu_HUD_Ref)) (delegate Custom|OnPressed_Event))))))

(event EventTick
  (params (DeltaSeconds :type Float%20%28single-precision%29)))

(fn ConstructionScript
  (|CallParentFunction))
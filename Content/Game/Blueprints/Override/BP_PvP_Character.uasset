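; PvP player character that fires a pistol on left click and loses health when damaged.
; Left click plays the fire montage and calls Shoot, which line-traces from the bullet trajectory point along the camera's forward vector.
; It spawns a bullet actor at the trace start, aimed at the impact point or trace end.
; ApplyDamage subtracts fixed bullet damage from Health; the Health and Bullets replication callbacks are empty.
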(event Custom|ApplyDamage
  (Variables|Default|SetHealth (- (Variables|Default|GetHealth) (Variables|Default|GetBULLET_DAMAGE))))

(event Custom|Shoot
  (bind _bullettrajectory (Variables|Default|GetBulletTrajectory))
  (bind _returnvalue (Transformation|GetWorldLocation _bullettrajectory))
  (bind _outhit (Collision|LineTraceByChannel _returnvalue (+ _returnvalue (* (Math|Vector|GetForwardVector (Variables|Default|GetFirstPersonCamera)) (Variables|Default|GetBULLET_RANGE))) "TraceTypeQuery1" false 0 "None" true "(R=1.000000,G=0.000000,B=0.000000,A=1.000000)" "(R=0.000000,G=1.000000,B=0.000000,A=1.000000)" 1.0))
  (if (.bBlockingHit (Collision|BreakHitResult _outhit))
    ;[0.15 0.15 0.15 0.5] Hit (pro gamer 1!1!!1!1!!)
    (Game|SpawnActorfromClass "/Game/Game/Blueprints/BP_Bullet.BP_Bullet_C" (Math|Transform|MakeTransform (.TraceStart (Collision|BreakHitResult _outhit)) (Math|Rotator|FindLookatRotation (.TraceStart (Collision|BreakHitResult _outhit)) (.ImpactPoint (Collision|BreakHitResult _outhit)))) "Undefined" "MultiplyWithRoot" 0 0)
    (else
      ;[0.15 0.15 0.15 0.5] No Hit (lol noob)
      (Game|SpawnActorfromClass "/Game/Game/Blueprints/BP_Bullet.BP_Bullet_C" (Math|Transform|MakeTransform (.TraceStart (Collision|BreakHitResult _outhit)) (Math|Rotator|FindLookatRotation (.TraceStart (Collision|BreakHitResult _outhit)) (.TraceEnd (Collision|BreakHitResult _outhit)))) "Undefined" "MultiplyWithRoot" 0 0))))

(event EventBeginPlay)

(event Collision|EventActorBeginOverlap
  (params (OtherActor :type Actor%20Object%20Reference)))

(event EventTick
  (params (DeltaSeconds :type Float%20%28single-precision%29)))

(event Input|MouseEvents|LeftMouseButton
  (params (Key :type Key%20Structure :default "None"))
  (:Pressed
    (Animation|Montage|PlayMontage (Variables|Character|GetMesh) "/Game/Characters/Mannequins/Anims/Pistol/MM_Pistol_Fire_Montage.MM_Pistol_Fire_Montage" 0.5
      (:then
        (CallFunction|Shoot)))))

(fn ConstructionScript
  (|CallParentFunction))

(fn OnRepHealth)

(fn OnRepBullets)
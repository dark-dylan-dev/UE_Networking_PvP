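; PvP player state that tracks kills, deaths and the win, lose or tie result of a match.
; Its events only set those variables; their OnRep functions forward changes to BP_PvP_Controller to update kill, death and HP UI or show end screens.
; Each OnRep targets player controller 0 without checking whether this state belongs to that player.
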(event Custom|AddLoseScreen
  (Variables|Default|SetIsWinner false))

(event Custom|AddWinScreen
  (Variables|Default|SetIsWinner true))

(event Custom|AddTieScreen
  (Variables|Default|SetIsTie true))

(event Custom|AddKill
  (Variables|Default|SetKills (+ (Variables|Default|GetKills) 1)))

(event Custom|AddDeath
  (Variables|Default|SetDeaths (+ (Variables|Default|GetDeaths) 1)))

(event EventBeginPlay
  (|CallParentFunction))

(fn ConstructionScript)

(fn OnRepKills
  (bind _asbp_pv_p_controller (Utilities|Casting|CastToBP_PvP_Controller (Game|GetPlayerController 0)))
  (Default|FuncUIAddKill _asbp_pv_p_controller))

(fn OnRepDeaths
  (bind _asbp_pv_p_controller (Utilities|Casting|CastToBP_PvP_Controller (Game|GetPlayerController 0)))
  (Default|FuncUIAddDeath _asbp_pv_p_controller)
  (Default|FuncUIModifyHP _asbp_pv_p_controller))

(fn OnRepIsLoser
  (if (not (Variables|Default|GetIsWinner))
    (bind _asbp_pv_p_controller (Utilities|Casting|CastToBP_PvP_Controller (Game|GetPlayerController 0)))
    (Default|AddLoseScreen _asbp_pv_p_controller)))

(fn OnRepIsWinner
  (bind _returnvalue (Game|GetPlayerController 0))
  (if (Variables|Default|GetIsWinner)
    (bind _asbp_pv_p_controller (Utilities|Casting|CastToBP_PvP_Controller _returnvalue))
    (Default|AddWinScreen _asbp_pv_p_controller)
    (else
      (bind _asbp_pv_p_controller_2 (Utilities|Casting|CastToBP_PvP_Controller _returnvalue))
      (Default|AddLoseScreen _asbp_pv_p_controller_2))))

(fn OnRepIsTie
  (bind _asbp_pv_p_controller (Utilities|Casting|CastToBP_PvP_Controller (Game|GetPlayerController 0)))
  (Default|FuncUITieScreen _asbp_pv_p_controller))
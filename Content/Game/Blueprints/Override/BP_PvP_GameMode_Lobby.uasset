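; Lobby game mode for PvP that moves the session to the Free For All map once enough players are present.
; A PlayersInLobby count drops on logout, and its RepNotify runs a listen ServerTravel when the count falls within the minimum and maximum bounds.
; The graph shown contains no logic that increments the count.
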(event EventBeginPlay)

(event EventTick
  (params (DeltaSeconds :type Float%20%28single-precision%29)))

(event EventOnLogout
  (params (ExitingController :type Controller%20Object%20Reference))
  (Variables|Default|SetPlayersInLobby (- (Variables|Default|GetPlayersInLobby) 1))
  (Development|PrintString "Disconnected"))

(fn ConstructionScript
  (|CallParentFunction))

(fn OnRepPlayersinLobby
  (if (and (>= (Variables|Default|GetPlayersInLobby) (Variables|Default|GetMIN_PLAYERS_IN_LOBBY)) (<= (Variables|Default|GetPlayersInLobby) (Variables|Default|GetMAX_PLAYERS_IN_LOBBY)))
    (Development|ExecuteConsoleCommand "ServerTravel /Game/Game/Maps/FreeForAll?listen" 0)
    (Development|PrintString "TravelToFFA")))
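; BP_PvP_GameMode_FFA is the game mode for free-for-all PvP matches.
; On BeginPlay it starts the match timer on BP_PvP_GameState, and a restart command server-travels to the Lobby map as a listen server.
; Respawn requests destroy the old character and restart the player at a randomly chosen PlayerStart.
; PostLogin is empty; logic copying the persistent name from the game instance to the player state is left disconnected.
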(event Custom|RequestRespawnCharacter
  (params (Controller :type BP%20Pv%20P%20Controller%20Object%20Reference) (Character :type BP%20Pv%20P%20Character%20Object%20Reference))
  (Actor|DestroyActor Character)
  (bind _outactors (Actor|GetAllActorsOfClass "/Script/Engine.PlayerStart"))
  (Class|GameModeBase|RestartPlayeratPlayerStart Controller (Utilities|Array|Get(acopy) _outactors (Math|Random|RandomIntegerinRange 0 (- (Utilities|Array|Length _outactors) 1)))))

(event Custom|RestartGameCommand
  (Development|ExecuteConsoleCommand "ServerTravel /Game/Game/Maps/Lobby?listen" 0))

(event EventBeginPlay
  (bind _asbp_pv_p_game_state (Utilities|Casting|CastToBP_PvP_GameState (Game|GetGameState)))
  (Default|StartTimer _asbp_pv_p_game_state))

(event EventPostLogin
  (params (NewPlayer :type Player%20Controller%20Object%20Reference)))

(fn ConstructionScript
  (|CallParentFunction))
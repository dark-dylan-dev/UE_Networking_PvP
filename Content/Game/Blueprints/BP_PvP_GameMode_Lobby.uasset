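; Lobby game mode for PvP that launches a free-for-all match when the player count is within limits.
; Logout decrements the PlayersInLobby count; no increment appears in these graphs.
; The count's RepNotify checks it against the lobby minimum and maximum, then server-travels to the FreeForAll map as a listen server and prints a launch message.
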(event EventOnLogout
  (params (ExitingController :type Controller%20Object%20Reference))
  (Variables|Default|SetPlayersInLobby (- (Variables|Default|GetPlayersInLobby) 1)))

(fn ConstructionScript
  (|CallParentFunction))

(fn OnRepPlayersinLobby
  (if (and (>= (Variables|Default|GetPlayersInLobby) (Variables|Default|GetMIN_PLAYERS_IN_LOBBY)) (<= (Variables|Default|GetPlayersInLobby) (Variables|Default|GetMAX_PLAYERS_IN_LOBBY)))
    (Development|ExecuteConsoleCommand "ServerTravel /Game/Game/Maps/FreeForAll?listen" 0)
    (Development|PrintString "Launching FFA Game..." true true "(R=1.000000,G=0.000000,B=0.000000,A=1.000000)" 3.0)))